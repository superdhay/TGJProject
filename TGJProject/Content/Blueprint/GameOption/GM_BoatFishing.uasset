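; Game mode for the boat fishing game that tracks score, player lives and the current recipe of random item IDs.
; A recipe is generated at BeginPlay and after each validation, growing from one to four entries as score passes fixed thresholds.
; ValidateRecipe awards points that double with each extra entry.
; LoseLife only decrements the life count, with no game-over check here.
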(event `self.ReceiveBeginPlay`
  (`self.GenerateRecipe`))

(event `LoseLife`
  (set `self.playerLife` (- (`self.playerLife`) 1)))

(event `ValidateRecipe`
  ;[1 1 1] Add recipe score to score
  (set `self.Score` (+ (`self.Score`) (`KismetMathLibrary.FTrunc` (`KismetMathLibrary.Conv_IntToDouble` (* (`self.pointsFor1`) (`KismetMathLibrary.FTrunc` (`KismetMathLibrary.MultiplyMultiply_FloatFloat` 2.0 (`KismetMathLibrary.Conv_IntToDouble` (`self.RecipeLenght`)))))))))
  (`self.GenerateRecipe`))

(fn `GenerateRecipe`
  (bind _currentrecipe (`self.currentRecipe`))
  (bind _currentrecipe_2 (`self.currentRecipe`))
  (bind _returnvalue (`KismetMathLibrary.RandomInteger` (`self.maxId`)))
  (`KismetArrayLibrary.Array_Clear` _currentrecipe)
  (`KismetArrayLibrary.Array_Add` _currentrecipe _returnvalue)
  (if (>= (`self.Score`) 100)
    (`KismetArrayLibrary.Array_Add` (`self.currentRecipe`) _returnvalue)
    (if (>= (`self.Score`) 500)
      (`KismetArrayLibrary.Array_Add` (`self.currentRecipe`) _returnvalue)
      (if (>= (`self.Score`) 2000)
        (`KismetArrayLibrary.Array_Add` _currentrecipe_2 _returnvalue))))
  (set `self.RecipeLenght` (`KismetArrayLibrary.Array_Length` _currentrecipe_2)))

(fn `UserConstructionScript`)