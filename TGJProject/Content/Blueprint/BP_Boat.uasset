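; Player-controlled fishing boat that records the ID of each fish overlapping its collider and checks the catch against the game mode's current recipe.
; The construction script hangs the hook at the line's length, and BeginPlay enables input and creates the UI widget.
; Pressing Jump jumps and runs the order-independent recipe check; any caught fish outside the recipe costs a life and generates a new recipe.
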(event `self.ReceiveBeginPlay`
  (bind _returnvalue (`GameplayStatics.GetPlayerController` 0))
  (`|ExecutionSequence`
    (:`then_0`
      (`self.EnableInput` _returnvalue))
    (:`then_1`
      (`|CreateWidget` "/Game/UI/W_UserInterface.W_UserInterface_C" _returnvalue))))

(event `InputAction|Jump`
  (params (Key :type "Key Structure"))
  (:`Pressed`
    (`self.Jump`)
    (`self.CheckRecipeFailed`)))

(event `self.Collider.OnComponentBeginOverlap`
  (params (OverlappedComponent :type "PrimitiveComponent Object Reference") (OtherActor :type "Actor Object Reference") (OtherComp :type "PrimitiveComponent Object Reference") (OtherBodyIndex :type Integer) (bFromSweep :type Boolean) (SweepResult :type "HitResult Structure (by ref)"))
  (bind (_asbp_fish _bsuccess) (cast `/Game/Blueprint/BP_Fish` OtherActor :!pure true))
  (if _bsuccess
    (`KismetArrayLibrary.Array_Add` (`self.FishedArray`) (`/Game/Blueprint/BP_Fish.Id` _asbp_fish))))

(fn `CheckRecipeFailed`
  (locals (isSameFish :type Boolean))
  (bind _fishedarray (`self.FishedArray`))
  (bind _asgm_boat_fishing (cast `/Game/Blueprint/GameOption/GM_BoatFishing` (`GameplayStatics.GetGameMode`) :!pure true))
  (bind _currentrecipe (`/Game/Blueprint/GameOption/GM_BoatFishing.currentRecipe` _asgm_boat_fishing))
  (if (`KismetArrayLibrary.Array_Contains` _currentrecipe (`|GetArrayItem` _fishedarray (- (`KismetArrayLibrary.Array_Length` _fishedarray) 1)))
    ;[1 1 1] Check if all array contains the fish (Ignore order)
    (for _array_element (`self.FishedArray`)
      (set `local.isSameFish` false)
      (for _array_element_2 _currentrecipe
        (if (== _array_element_2 _array_element)
          (set `local.isSameFish` true)))
      (if (not (`local.isSameFish`))
        (break)))
    (if (not (`local.isSameFish`))
      ;[1 1 1] Lose a life and refresh a new Recipe
      (`/Game/Blueprint/GameOption/GM_BoatFishing.LoseLife` _asgm_boat_fishing :!label _label)
      (`/Game/Blueprint/GameOption/GM_BoatFishing.GenerateRecipe` _asgm_boat_fishing))
    (else
      (goto _label))))

(fn `UserConstructionScript`
  (set `ArrowComponent.ArrowLength` (`self.fishingLineLength`) (`self.fishingLine`))
  (`SceneComponent.K2_AddLocalOffset` (`self.fishingHook`) (`KismetMathLibrary.MakeVector` 0.0 0.0 (* -1 (`ArrowComponent.ArrowLength` (`self.fishingLine`)))) false false))