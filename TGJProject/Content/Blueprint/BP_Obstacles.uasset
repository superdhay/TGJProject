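; Obstacle actor that slides its Obstacle component along world Y and can randomize its look.
; BeginPlay plays the ObstacleMovement timeline, whose updates lerp Y from the current position toward a fixed target by timeline alpha times delta seconds, easing rather than following a fixed path.
; A separate SetObstacle event applies a random material from the Obstacles array; nothing in this graph calls it.
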(event `self.ReceiveBeginPlay`
  (bind (_direction _alpha) (`Timeline|ObstacleMovement`)
    (:`Update`
      (`SceneComponent.K2_SetWorldLocation` (`self.Obstacle`) (`KismetMathLibrary.MakeVector` (.x (`SceneComponent.K2_GetComponentLocation` (`self.Obstacle`))) (`KismetMathLibrary.Lerp` (.y (`SceneComponent.K2_GetComponentLocation` (`self.Obstacle`))) 2000.0 (* _alpha (`GameplayStatics.GetWorldDeltaSeconds`))) (.z (`SceneComponent.K2_GetComponentLocation` (`self.Obstacle`)))) false false))))

(event `SetObstacle`
  (bind _obstacles (`self.Obstacles`))
  (`PrimitiveComponent.SetMaterial` (`self.Obstacle`) 0 (`|GetArrayItem` _obstacles (`KismetMathLibrary.RandomIntegerInRange` 0 (- (`KismetArrayLibrary.Array_Length` _obstacles) 1)))))

(fn `UserConstructionScript`)