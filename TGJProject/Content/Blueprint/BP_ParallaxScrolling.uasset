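; Parallax background actor that scrolls three background layers through their materials.
; The construction script creates a dynamic material instance for each layer from its own source material.
; On BeginPlay, if IsReady is set, the Scrolling timeline plays at a rate of ParallaxVelocity.
; Each update adds velocity-scaled delta time to the timeline alpha, wraps values above one and writes the same Offset parameter to all three materials.
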(event `self.ReceiveBeginPlay`
  (if (`self.bIsReady?`)
    (`TimelineComponent.SetPlayRate` (`self.Scrolling`) (`self.ParallaxVelocity`))
    (bind (_direction _alpha) (`Timeline|Scrolling`)
      (:`Update`
        (set `self.ParallaxOffset` (+ _alpha (* (`GameplayStatics.GetWorldDeltaSeconds`) (`self.ParallaxVelocity`))))
        (if (> (`self.ParallaxOffset`) 1.0)
          (set `self.ParallaxOffset` (`KismetMathLibrary.FMod` (`self.ParallaxOffset`) 1.0)))
        (`MaterialInstanceDynamic.SetScalarParameterValue` (`self.BackgroundMID_01`) "Offset" (`self.ParallaxOffset`))
        (`MaterialInstanceDynamic.SetScalarParameterValue` (`self.BackgroundMID_02`) "Offset" (`self.ParallaxOffset`))
        (`MaterialInstanceDynamic.SetScalarParameterValue` (`self.BackgroundMID_03`) "Offset" (`self.ParallaxOffset`))))))

(fn `UserConstructionScript`
  (`|ExecutionSequence`
    (:`then_0`
      (bind _returnvalue (`PrimitiveComponent.CreateDynamicMaterialInstance` (`self.Background_01`) 0 "/Game/Material/MI_Background_01.MI_Background_01" "None"))
      (set `self.BackgroundMID_01` _returnvalue))
    (:`then_1`
      (bind _returnvalue_2 (`PrimitiveComponent.CreateDynamicMaterialInstance` (`self.Background_02`) 0 "/Game/Material/MI_Background_02.MI_Background_02" "None"))
      (set `self.BackgroundMID_02` _returnvalue_2))
    (:`then_2`
      (bind _returnvalue_3 (`PrimitiveComponent.CreateDynamicMaterialInstance` (`self.Background_03`) 0 "/Game/Material/MI_Background_03.MI_Background_03" "None"))
      (set `self.BackgroundMID_03` _returnvalue_3))))