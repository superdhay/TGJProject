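; BP_GenerateObstackes is a spawner actor that creates BP_Obstacles throughout play and destroys any that overlap its Box.
; From BeginPlay it loops endlessly, spawning one obstacle, calling SetObstacle on it, then waiting a random whole number of seconds.
; The construction script derives Z from the Generator's scale.
; CalculateSpawnObstacles supplies the spawn transform, though its MakeTransform using Generator position and offset Z is left unconnected.
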(event `self.ReceiveBeginPlay`
  (for _ (range 1) :!label _label
    (bind _returnvalue (`|SpawnActorFromClass` "/Game/Blueprint/BP_Obstacles.BP_Obstacles_C" (`KismetMathLibrary.MakeTransform` (`KismetMathLibrary.MakeVector` (.x (`SceneComponent.K2_GetComponentLocation` (`self.Generator`))) (.y (`SceneComponent.K2_GetComponentLocation` (`self.Generator`))) (+ (`self.Z`) 400.0))) "Undefined" "OverrideRootScale" null null))
    (`/Game/Blueprint/BP_Obstacles.SetObstacle` _returnvalue))
  (`KismetSystemLibrary.Delay` (`KismetMathLibrary.Conv_IntToDouble` (`KismetMathLibrary.RandomIntegerInRange` 1 10)))
  (goto _label))

(event `self.Box.OnComponentBeginOverlap`
  (params (OverlappedComponent :type "PrimitiveComponent Object Reference") (OtherActor :type "Actor Object Reference") (OtherComp :type "PrimitiveComponent Object Reference") (OtherBodyIndex :type Integer) (bFromSweep :type Boolean) (SweepResult :type "HitResult Structure (by ref)"))
  (bind (_asbp_obstacles _bsuccess) (cast `/Game/Blueprint/BP_Obstacles` OtherActor :!pure true))
  (if _bsuccess
    (`self.K2_DestroyActor` _asbp_obstacles)))

(fn `UserConstructionScript`
  (set `self.Z` (* (.z (`SceneComponent.RelativeScale3D` (`self.Generator`))) 100.0)))