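; BP_FishSpawn is a spawner actor that creates a single BP_Fish when play begins.
; The construction script stores the Cube component's world X and Y scale.
; BeginPlay picks random X and Y values between the Cube's world location and those raw scale values, rather than bounds offset from its location.
; Spawn height comes from the Cube's Z scale plus a small offset, ignoring its world Z position.
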(event `self.ReceiveBeginPlay`
  (bind _cube (`self.Cube`))
  (`|SpawnActorFromClass` "/Game/Blueprint/BP_Fish.BP_Fish_C" (`KismetMathLibrary.MakeTransform` (`KismetMathLibrary.MakeVector` (`KismetMathLibrary.RandomFloatInRange` (.x (`SceneComponent.K2_GetComponentLocation` _cube)) (`self.X`)) (`KismetMathLibrary.RandomFloatInRange` (.y (`SceneComponent.K2_GetComponentLocation` _cube)) (`self.Y`)) (+ (.z (`SceneComponent.K2_GetComponentScale` _cube)) 3.0))) "Undefined" "OverrideRootScale" null null))

(fn `UserConstructionScript`
  (set `self.X` (.x (`SceneComponent.K2_GetComponentScale` (`self.Cube`))))
  (set `self.Y` (.y (`SceneComponent.K2_GetComponentScale` (`self.Cube`)))))